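; Health Blueprint that tracks a clamped health value and exposes it as a fraction of MaxHealth.
; TakeDamage subtracts damage and calls HealthEmpty at zero, otherwise calls TakeDamage with the damage amount.
; Invulnerability looks unfinished: RemoveInvuln clears IsInvulnerable, but TakeDamage neither checks that flag nor uses its InvulnTime input.
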(fn `GetHealthPercentage`
  (returns (`Health Percentage` :type "Float (double-precision)"))
  (return (/ (`self.Health`) (`self.MaxHealth`))))

(fn `RemoveInvuln`
  (set `self.is Invulnerable` false))

(fn `Take Damage`
  (params (Damage :type "Float (double-precision)") (`Invuln Time` :type "Float (double-precision)" :default -1.0))
  (bind _output_get (set `self.Health` (`KismetMathLibrary.FClamp` (- (`self.Health`) Damage) 0.0 (`self.MaxHealth`))))
  (if (== _output_get 0.0)
    (`self.HealthEmpty`)
    (else
      (`self.TakeDamage` Damage))))